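; Gameplay ability for the Fireball that commits, plays a montage and ends when the montage completes, blends out or is stopped.
; Once the montage starts, it waits for a single damage gameplay event, and it ends both stored tasks on ability end.
; Nothing handles the received event: the nodes applying a set-by-caller damage effect to the target and printing debug names are disconnected, so the ability deals no damage itself.
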(event Ability|EventActivateAbility
  (bind _returnvalue (Ability|CommitAbility))
  (if _returnvalue
    (bind _asynctaskproxy (|PlayMontageandWaitProxy "None" (Variables|Default|GetMontage%20to%20Play) 1.0 "None" true 1.0 0.0 false)
      (:then
        (Variables|Default|SetMontageTask _asynctaskproxy)
        (bind (_asynctaskproxy_2 _payload) (Ability|Tasks|WaitGameplayEvent "(TagName=\"Event.Damage\")" 0 true)
          (:then
            (Variables|Default|SetGameplayEventTask _asynctaskproxy_2))))
      (:OnCompleted
        (Ability|EndAbility :!label _label))
      (:OnBlendOut
        (goto _label))
      (:OnInterrupted
        (goto _label))
      (:OnCancelled
        (goto _label)))
    (else
      (Ability|EndAbility))))

(event Ability|EventOnEndAbility
  (params (bWasCancelled :type Boolean))
  (bind _montagetask (Variables|Default|GetMontageTask))
  (bind _gameplayeventtask (Variables|Default|GetGameplayEventTask))
  (if (Utilities|IsValid _montagetask)
    (GameplayTasks|EndTask _montagetask))
  (if (Utilities|IsValid _gameplayeventtask)
    (GameplayTasks|EndTask _gameplayeventtask)))