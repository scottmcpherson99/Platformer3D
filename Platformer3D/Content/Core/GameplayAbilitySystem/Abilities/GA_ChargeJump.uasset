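; Gameplay ability for a charged jump: holding input flags the character as preparing to jump, and releasing launches it.
; Hold time, scaled and clamped to a range, drives jump height and duration, while forward distance stays fixed.
; A root motion jump force task follows the avatar's facing and ends the ability on finish or landing.
; Ending the ability also ends any valid input or jump task.
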(event Ability|EventActivateAbility
  (bind (_asynctaskproxy _timeheld) (Ability|Tasks|WaitInputRelease false)
    (:then
      (Variables|Default|SetWaitInputReleaseTask _asynctaskproxy)
      (bind _asbase_character (Utilities|Casting|CastToBaseCharacter (Ability|GetAvatarActorfromActorInfo)))
      (bind _output_get (Variables|Default|SetCharacterRef _asbase_character))
      (Variables|/Script/Platformer3D.BaseCharacter|SetbPreparingToJump _output_get true))
    (:OnRelease
      (Variables|/Script/Platformer3D.BaseCharacter|SetbPreparingToJump (Variables|Default|GetCharacterRef) false)
      (bind _asynctaskproxy_2 (|ApplyRootMotionJumpForce "None" (Transformation|GetActorRotation (Ability|GetAvatarActorfromActorInfo)) 5e+02 (* (Math|Float|Max(Float) (Math|Float|Min(Float) (* _timeheld 1.5) 1e+01) 4.0) 3e+02) (* (Math|Float|Max(Float) (Math|Float|Min(Float) (* _timeheld 1.5) 1e+01) 4.0) 0.35) 0.0 true "MaintainLastRootMotionVelocity" "0, 0, 0" 0.0)
        (:then
          (Variables|Default|SetJumpTask _asynctaskproxy_2))
        (:OnFinish
          (Ability|EndAbility :!label _label))
        (:OnLanded
          (goto _label))))))

(event Ability|EventOnEndAbility
  (params (bWasCancelled :type Boolean))
  (bind _waitinputreleasetask (Variables|Default|GetWaitInputReleaseTask))
  (bind _jumptask (Variables|Default|GetJumpTask))
  (if (Utilities|IsValid _waitinputreleasetask)
    (GameplayTasks|EndTask _waitinputreleasetask))
  (if (Utilities|IsValid _jumptask)
    (GameplayTasks|EndTask _jumptask)))