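; Gameplay ability that makes the avatar dash along its forward vector with a dodge roll animation, provided CommitAbility succeeds (noted as a mana check).
; A root motion constant force task drives the movement while a montage task plays the roll alongside it.
; The montage completing, blending out, being interrupted or cancelled ends the ability, and OnEndAbility stops both stored tasks.
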(event Ability|EventActivateAbility
  ;[1 1 1] check if we can spend the mana
  (bind _returnvalue (Ability|CommitAbility))
  (if _returnvalue
    (bind _asynctaskproxy (Ability|Tasks|ApplyRootMotionConstantForce "None" (Transformation|GetActorForwardVector (Ability|GetAvatarActorfromActorInfo)) 1.75e+03 1.63 false 0 "MaintainLastRootMotionVelocity")
      (:then
        (Variables|Default|SetRootMotionTask _asynctaskproxy)
        (bind _asynctaskproxy_2 (|PlayMontageandWaitProxy "None" "/Game/Assets/Characters/Player/Animations/Montages/MM_Player_DodgeRoll_Montage.MM_Player_DodgeRoll_Montage" 1.0 "None" true 1.0 0.0 false)
          (:then
            (Variables|Default|SetMontageTask _asynctaskproxy_2))
          (:OnCompleted
            (Ability|EndAbility :!label _label))
          (:OnBlendOut
            (goto _label))
          (:OnInterrupted
            (goto _label))
          (:OnCancelled
            (goto _label)))))
    (else
      ;[1 1 1] end ability, not enough mana
      (Ability|EndAbility))))

(event Ability|EventOnEndAbility
  (params (bWasCancelled :type Boolean))
  (bind _rootmotiontask (Variables|Default|GetRootMotionTask))
  (bind _montagetask (Variables|Default|GetMontageTask))
  (if (Utilities|IsValid _rootmotiontask)
    (GameplayTasks|EndTask _rootmotiontask))
  (if (Utilities|IsValid _montagetask)
    (GameplayTasks|EndTask _montagetask)))