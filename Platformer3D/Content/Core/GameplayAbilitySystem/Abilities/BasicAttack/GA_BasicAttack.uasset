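; GA_BasicAttack is a Gameplay Ability that plays an attack montage and deals damage.
; After committing the ability, it plays the montage and waits for a single Event.Damage gameplay event.
; That event applies GE_DealDamage from instigator to target, passing Damage as a SetByCaller magnitude.
; It ends when the commit fails or the montage finishes, blends out or is interrupted, stopping both tasks.
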(event Ability|EventActivateAbility
  ;[1 1 1] check if we can spend the mana
  (bind _returnvalue (Ability|CommitAbility))
  (if _returnvalue
    ;[1 1 1] play attack montage
    (bind _asynctaskproxy (|PlayMontageandWaitProxy "None" (Variables|Default|GetMontage%20to%20Play) 1.0 "None" true 1.0 0.0 false)
      (:then
        (Variables|Default|SetMontageTask _asynctaskproxy)
        (bind (_asynctaskproxy_2 _payload) (Ability|Tasks|WaitGameplayEvent "(TagName=\"Event.Damage\")" 0 true)
          (:then
            (Variables|Default|SetGameplayEventTask _asynctaskproxy_2))
          (:EventReceived
            (bind _result (Math|Float|NegateFloat (Variables|Default|GetDamage))
              (:%20%20
                (bind _returnvalue_2 (Ability|GameplayEffect|AssignTagSetbyCallerMagnitude (Ability|MakeOutgoingGameplayEffectSpec "/Game/Core/GameplayAbilitySystem/Effects/GE_DealDamage.GE_DealDamage_C") "(TagName=\"Event.Damage\")" _result))
                (GameplayEffects|ApplyGameplayEffectSpecToTarget (Ability|GetAbilitySystemComponent (.Instigator (Utilities|Struct|BreakGameplayEventData _payload))) _returnvalue_2 (Ability|GetAbilitySystemComponent (.Target (Utilities|Struct|BreakGameplayEventData _payload)))))))))
      (:OnCompleted
        (Ability|EndAbility :!label _label))
      (:OnBlendOut
        (goto _label))
      (:OnInterrupted
        (goto _label))
      (:OnCancelled
        (goto _label)))
    (else
      ;[1 1 1] end ability, not enough mana
      (Ability|EndAbility))))

(event Ability|EventOnEndAbility
  (params (bWasCancelled :type Boolean))
  (bind _montagetask (Variables|Default|GetMontageTask))
  (bind _gameplayeventtask (Variables|Default|GetGameplayEventTask))
  (if (Utilities|IsValid _montagetask)
    (GameplayTasks|EndTask _montagetask))
  (if (Utilities|IsValid _gameplayeventtask)
    (GameplayTasks|EndTask _gameplayeventtask)))