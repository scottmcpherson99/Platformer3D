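; GA_HealingRegen is a gameplay ability that makes the owner play a heal animation and gain a regeneration effect.
; On activation it commits the ability, starts the heal montage task and immediately applies GE_Regen to the owner, ending right away if the commit fails.
; The ability ends when the montage completes, blends out or is interrupted, and OnEndAbility ends the stored montage task if still valid.
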(event Ability|EventActivateAbility
  (bind _returnvalue (Ability|CommitAbility))
  (if _returnvalue
    (bind _asynctaskproxy (|PlayMontageandWaitProxy "None" "/Game/Assets/Characters/Player/Animations/Montages/MM_Player_Heal_Montage.MM_Player_Heal_Montage" 1.0 "None" true 1.0 0.0 false)
      (:then
        (Variables|Default|SetMontageTask _asynctaskproxy)
        (Ability|ApplyGameplayEffectToOwner "/Game/Core/GameplayAbilitySystem/Effects/GE_Regen.GE_Regen_C"))
      (:OnCompleted
        (Ability|EndAbility :!label _label))
      (:OnBlendOut
        (goto _label))
      (:OnInterrupted
        (goto _label)))
    (else
      (Ability|EndAbility))))

(event Ability|EventOnEndAbility
  (params (bWasCancelled :type Boolean))
  (bind _montagetask (Variables|Default|GetMontageTask))
  (if (Utilities|IsValid _montagetask)
    (GameplayTasks|EndTask _montagetask)))