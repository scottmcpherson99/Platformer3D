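; Player character Blueprint that drives dash, basic attack and other abilities through the Gameplay Ability System.
; BeginPlay grants starting abilities with array indices as input IDs; Left Ctrl presses and releases the ID from AbilityToDo.
; Left Shift and left mouse activate dash and basic attack by class.
; DoBasicAttack sphere-traces forward from the right hand and sends itself a damage gameplay event targeting each hit actor.
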(event EventBeginPlay
  (for (_array_element _array_index) (Variables|Default|GetAbilitiesOnStart)
    (GameplayAbilities|GiveAbility (Variables|Default|GetAbilitySystemComponent) _array_element 0 _array_index)))

(event Collision|EventActorBeginOverlap
  (params (OtherActor :type Actor%20Object%20Reference)))

(event EventDoBasicAttack
  (bind _mesh (Variables|Character|GetMesh))
  (bind _returnvalue (Transformation|GetSocketLocation _mesh "RightHand"))
  (bind _outhits (Collision|MultiSphereTraceByChannel _returnvalue (+ _returnvalue (* (Math|Vector|GetForwardVector (Transformation|GetActorRotation)) (Variables|Default|GetSpellRange))) 1e+01 "TraceTypeQuery2" false (Utilities|Array|MakeArray self) "None"))
  (for _array_element _outhits
    (Ability|SendGameplayEventtoActor self "(TagName=\"Event.Damage\")" (Utilities|Struct|MakeGameplayEventData "(TagName=\"Event.Damage\")" self (.hitactor _array_element)))))

(event EventTick
  (params (DeltaSeconds :type Float%20%28single-precision%29)))

(event Input|MouseEvents|LeftMouseButton
  (params (Key :type Key%20Structure :default "None"))
  (:Pressed
    (Abilities|TryActivateAbilitybyClass (Variables|Default|GetAbilitySystemComponent) "/Game/Core/GameplayAbilitySystem/Abilities/GA_BasicAttack.GA_BasicAttack_C" true)))

(event Input|KeyboardEvents|LeftCtrl
  (params (Key :type Key%20Structure :default "None"))
  (:Pressed
    (Class|AbilitySystemComponent|PressInputID (Variables|Default|GetAbilitySystemComponent) (Math|Conversions|ToInteger(Byte) (Variables|Default|GetAbilityToDo))))
  (:Released
    (Class|AbilitySystemComponent|ReleaseInputID (Variables|Default|GetAbilitySystemComponent) (Math|Conversions|ToInteger(Byte) (Variables|Default|GetAbilityToDo)))))

(event Input|KeyboardEvents|LeftShift
  (params (Key :type Key%20Structure :default "None"))
  (:Pressed
    (Abilities|TryActivateAbilitybyClass (Variables|Default|GetAbilitySystemComponent) "/Game/Core/GameplayAbilitySystem/Abilities/GA_Dash.GA_Dash_C" true)))

(fn ConstructionScript)